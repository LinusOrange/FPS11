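; Server-authoritative melee enemy that chases first-person player characters and adds team score to the game state when destroyed.
; A looping timer scans for players and AI-moves to ClosestTarget; ClosestDist is never reset between scans.
; A second timer damages that target within range, followed by a cooldown.
; The damage handler sets health to Damage minus EnemyHealth (reversed subtraction), destroying the enemy at zero or below.
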(event Custom|DoMoveToTarget
  (Networking|SwitchHasAuthority
    (:Authority
      (AI|AIMoveTo self "0, 0, 0" (Variables|Default|GetClosestTarget) 1e+02 false))))

(event Custom|Try%20Attack
  (if (Variables|Default|GetbCanAttack)
    (Utilities|IsValid (Variables|Default|GetClosestTarget)
      (:Is%20Valid
        (if (<= (Math|Vector|Distance(Vector) (Transformation|GetActorLocation) (Transformation|GetActorLocation (Variables|Default|GetClosestTarget))) (Variables|Default|GetAttackRange))
          (Game|Damage|ApplyDamage (Variables|Default|GetClosestTarget) (Variables|Default|GetAttackDamage) (Pawn|GetController) self)
          (Variables|Default|SetbCanAttack false)
          (Utilities|FlowControl|Delay (Variables|Default|GetAttackCD))
          (Variables|Default|SetbCanAttack true))))))

(event EventBeginPlay
  (Networking|SwitchHasAuthority
    (:Authority
      (Utilities|FlowControl|Sequence
        (:then_0
          (Utilities|Time|SetTimerbyFunctionName 0 "UpdateMove" 0.3 true))
        (:then_1
          (Utilities|Time|SetTimerbyEvent (delegate Custom|Try%20Attack) 0.2 true))))))

(event Game|Damage|EventAnyDamage
  (params (Damage :type Float%20%28single-precision%29) (DamageType :type Damage%20Type%20Object%20Reference) (InstigatedBy :type Controller%20Object%20Reference) (DamageCauser :type Actor%20Object%20Reference))
  (Networking|SwitchHasAuthority
    (:Authority
      (bind _output_get (Variables|Default|SetEnemyHealth (- Damage (Variables|Default|GetEnemyHealth))))
      (if (<= _output_get 0.0)
        (bind _asbp_mygamestate (Utilities|Casting|CastToBP_mygamestate (Game|GetGameState)))
        (Default|AddScore _asbp_mygamestate 10)
        (bind _asbp_mygamestate_2 (Utilities|Casting|CastToBP_mygamestate (Game|GetGameState)))
        (Development|PrintString (Utilities|String|ToString(Text) (Utilities|Text|FormatText "Score = {s}" (Variables|/Game/BP_mygamestate.BP_mygamestate_C|GetTeamScore _asbp_mygamestate_2))))
        (Actor|DestroyActor)))))

(fn ConstructionScript)

(fn UpdateMove
  (bind _outactors (Actor|GetAllActorsOfClass "/Game/FirstPerson/Blueprints/BP_FirstPersonCharacter.BP_FirstPersonCharacter_C"))
  (for _array_element _outactors
    (Utilities|Casting|CastToBP_FirstPersonCharacter _array_element)
    (if (< (Math|Vector|Distance(Vector) (Transformation|GetActorLocation _array_element) (Transformation|GetActorLocation)) (Variables|Default|GetClosestDist))
      (Utilities|FlowControl|Sequence
        (:then_0
          (Variables|Default|SetClosestDist (Math|Vector|Distance(Vector) (Transformation|GetActorLocation _array_element) (Transformation|GetActorLocation))))
        (:then_1
          (Variables|Default|SetClosestTarget _array_element)))))
  (CallFunction|DoMovetoTarget))

(fn TryAttack
  (if (Variables|Default|GetbCanAttack)
    (Utilities|IsValid (Variables|Default|GetClosestTarget)
      (:Is%20Valid
        (if (<= (Math|Vector|Distance(Vector) (Transformation|GetActorLocation) (Transformation|GetActorLocation (Variables|Default|GetClosestTarget))) (Variables|Default|GetAttackRange))
          (Game|Damage|ApplyDamage (Variables|Default|GetClosestTarget) (Variables|Default|GetAttackDamage) (Pawn|GetController) self)
          (Variables|Default|SetbCanAttack false)
          (Utilities|Time|SetTimerbyEvent 0 (Variables|Default|GetAttackCD)))))))